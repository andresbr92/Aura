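; GA_FireBolt is the gameplay ability that casts a fire bolt projectile along the avatar's camera direction.
; On activation it caches the camera forward vector, sets the facing target and plays the cast montage.
; On the montage's gameplay event, the authority spawns BP_FireBolt at the combat socket, using only yaw and roll, with a level-scaled SetByCaller damage spec.
; The ability ends when the montage blends out.
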(event `self.K2_ActivateAbility`
  (bind (_owneractor _avataractor) (break `GameplayAbilityActorInfo` (`self.GetActorInfo`)))
  (bind (_returnvalue_roll _returnvalue_pitch _returnvalue_yaw) (`KismetMathLibrary.BreakRotator` (`KismetMathLibrary.Conv_VectorToRotator` (`self.LookingAt`))))
  (bind _returnvalue (`AbilitySystemBlueprintLibrary.GetAbilitySystemComponent` _avataractor))
  (bind _ascombat_interface (cast `CombatInterface` _avataractor))
  (set `self.As Combat Interface` _ascombat_interface)
  (`|ExecutionSequence`
    (:`then_0`
      ;[1 1 1] Utility for projectile
      (bind _returnvalue_2 (`CombatInterface.GetCameraForwardVector` (`self.As Combat Interface`)))
      (set `self.LookingAt` _returnvalue_2))
    (:`then_1`
      (`CombatInterface.SetFacingTarget` (`self.As Combat Interface`)))
    (:`then_2`
      (`AbilityTask_PlayMontageAndWait.CreatePlayMontageAndWaitProxy` "None" "/Game/Assets/Characters/Aura/Animations/Abilities/AM_Cast_FireBolt.AM_Cast_FireBolt"
        (:`then`
          (`AbilityTask_WaitGameplayEvent.WaitGameplayEvent` (struct :`TagName` "Event.Montage.FireBolt") null
            (:`EventReceived`
              (`self.K2_HasAuthority`
                (:`True`
                  (bind _returnvalue_3 (`CombatInterface.GetCombatSocketLocation` (`self.As Combat Interface`)))
                  (bind _output_get (set `self.ProjectileSpawnLocation` _returnvalue_3))
                  ;[1 1 1] Also done in c++
                  (bind _returnvalue_4 (`AbilitySystemBlueprintLibrary.AssignTagSetByCallerMagnitude` (`AbilitySystemComponent.MakeOutgoingSpec` _returnvalue "/Game/Blueprints/AbilitySystem/GameplayEffects/GE_BasicDamage.GE_BasicDamage_C" 1.0 (`AbilitySystemComponent.MakeEffectContext` _returnvalue)) (struct :`TagName` "Damage") (`self.GetDamageByAbilityLevel` 11.0)))
                  (`GameplayTask_SpawnActor.SpawnActor` null _output_get (`KismetMathLibrary.MakeRotator` _returnvalue_roll 0.0 _returnvalue_yaw) "/Game/Blueprints/AbilitySystem/GameplayAbilities/Fire/FireBolt/BP_FireBolt.BP_FireBolt_C" false _returnvalue_4 null))))))
        (:`OnBlendOut`
          (`self.K2_EndAbility`))))))