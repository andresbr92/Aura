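; BP_EnemyBase is the base enemy character Blueprint, handling its health bar hookup and dissolve effects.
; On BeginPlay it casts the HealthBar widget component's widget to AuraUserWidget and sets the enemy itself as that widget's controller.
; The StartDissolvingCharacter and StartDissolvingWeapon events each play their own timeline, driving the Dissolve scalar parameter on the dynamic material instance passed in.
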(event `self.StartDissolvingCharacter`
  (params (MaterialInstanceDynamic :type "MaterialInstanceDynamic Object Reference"))
  (bind (_direction _dissolve_parametter) (`Timeline|Timeline`)
    (:`Update`
      (`MaterialInstanceDynamic.SetScalarParameterValue` MaterialInstanceDynamic "Dissolve" _dissolve_parametter))))

(event `self.StartDissolvingWeapon`
  (params (MaterialInstanceDynamic :type "MaterialInstanceDynamic Object Reference"))
  (bind (_direction _dissolve_parametter) (`Timeline|Timeline_0`)
    (:`Update`
      (`MaterialInstanceDynamic.SetScalarParameterValue` MaterialInstanceDynamic "Dissolve" _dissolve_parametter))))

(event `self.ReceiveBeginPlay`
  (bind _asaura_user_widget (cast `AuraUserWidget` (`WidgetComponent.GetUserWidgetObject` (`self.HealthBar`))))
  (`AuraUserWidget.SetWidgetController` _asaura_user_widget self))

(event `self.ReceiveTick`
  (params (DeltaSeconds :type "Float (single-precision)")))

(fn `UserConstructionScript`)